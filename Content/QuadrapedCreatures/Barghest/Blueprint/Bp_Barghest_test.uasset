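; Test Barghest enemy creature that chases the player, deals damage and dies when its health runs out.
; A Findplayer overlap or PawnSensing sighting starts an AI MoveTo toward the target, and the attack hitbox applies damage to overlapping player-tagged actors.
; Only damage from player-tagged causers lowers Hp.
; At zero it clears the master pose, plays the death animation on mesh, tail and hair, then destroys itself after a delay.
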(event OnComponentBeginOverlap(findplayer)
  (params (OverlappedComponent :type Primitive%20Component%20Object%20Reference) (OtherActor :type Actor%20Object%20Reference) (OtherComp :type Primitive%20Component%20Object%20Reference) (OtherBodyIndex :type Integer) (bFromSweep :type Boolean) (SweepResult :type Hit%20Result%20Structure%20%28by%20ref%29))
  ;[1 1 1] sencor of find player
  (if (Actor|ActorHasTag OtherActor "player")
    (Development|PrintString "find player from bp_barghest")
    (bind _ascharacter (Utilities|Casting|CastToCharacter (Game|Player|GetPlayerPawn 0)))
    (AI|AIMoveTo self "0, 0, 0" _ascharacter 5.0 false)))

(event OnComponentBeginOverlap(atk_hit_box)
  (params (OverlappedComponent :type Primitive%20Component%20Object%20Reference) (OtherActor :type Actor%20Object%20Reference) (OtherComp :type Primitive%20Component%20Object%20Reference) (OtherBodyIndex :type Integer) (bFromSweep :type Boolean) (SweepResult :type Hit%20Result%20Structure%20%28by%20ref%29))
  ;[1 1 1] attack collision
  (if (Actor|ActorHasTag OtherActor "player")
    (if (!= OtherActor self)
      (Game|Damage|ApplyDamage OtherActor 1e+01 0 self "/Script/Engine.DamageType"))))

(event OnSeePawn(PawnSensing)
  (params (Pawn :type Pawn%20Object%20Reference))
  (bind _ascharacter (Utilities|Casting|CastToCharacter Pawn))
  (AI|AIMoveTo self "0, 0, 0" _ascharacter 5.0 false))

(event EventBeginPlay)

(event Game|Damage|EventAnyDamage
  (params (Damage :type Float%20%28single-precision%29) (DamageType :type Damage%20Type%20Object%20Reference) (InstigatedBy :type Controller%20Object%20Reference) (DamageCauser :type Actor%20Object%20Reference))
  ;[1 1 1] dmg input
  (if (Actor|ActorHasTag DamageCauser "player")
    (Variables|Default|Sethp (- (Variables|Default|Gethp) Damage))
    (if (<= (Variables|Default|Gethp) 0.0)
      ;;[1 1 1] change to play animation here
      (Development|PrintString "Play dead animation from bp_barghest")
      (Class|SkinnedMeshComponent|SetMasterPoseComponent (Variables|Character|GetMesh) 0 false)
      (Components|Animation|PlayAnimation (Variables|Character|GetMesh) "/Game/QuadrapedCreatures/Barghest/Animations/BARGHEST_deathNormal.BARGHEST_deathNormal" false)
      (Utilities|FlowControl|Delay 2.0)
      (Actor|DestroyActor)
      (else
        (Development|PrintString "wolf get dmg from bp_barghest")
        (Development|PrintString (Utilities|String|ToString(Float) (Variables|Default|Gethp)))))))

(event EventTick
  (params (DeltaSeconds :type Float%20%28single-precision%29)))

(event Collision|EventActorBeginOverlap
  (params (OtherActor :type Actor%20Object%20Reference)))

(fn ConstructionScript)