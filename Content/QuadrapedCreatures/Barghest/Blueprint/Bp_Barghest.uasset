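; Barghest enemy creature that wanders the navmesh, chases and bites the player, and destroys itself after a death animation.
; Overlap volumes set detection and attack-range flags, which Tick reads to choose between random roaming, AI MoveTo chase and attack.
; Delays time the bite hitbox and cooldown behind a StopEvent gate, with animations played directly on hair, body and tail meshes.
; Only damage from player-tagged causers lowers Hp.
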(event OnComponentBeginOverlap(findplayer)
  (params (OverlappedComponent :type Primitive%20Component%20Object%20Reference) (OtherActor :type Actor%20Object%20Reference) (OtherComp :type Primitive%20Component%20Object%20Reference) (OtherBodyIndex :type Integer) (bFromSweep :type Boolean) (SweepResult :type Hit%20Result%20Structure%20%28by%20ref%29))
  ;[1 1 1] sencor of find player
  (if (Actor|ActorHasTag OtherActor "player")
    (Variables|Default|Setfind%20player? true)))

(event OnComponentBeginOverlap(atk_hit_box)
  (params (OverlappedComponent :type Primitive%20Component%20Object%20Reference) (OtherActor :type Actor%20Object%20Reference) (OtherComp :type Primitive%20Component%20Object%20Reference) (OtherBodyIndex :type Integer) (bFromSweep :type Boolean) (SweepResult :type Hit%20Result%20Structure%20%28by%20ref%29))
  ;[1 1 1] attack collision
  (if (Actor|ActorHasTag OtherActor "player")
    (if (!= OtherActor self)
      (Game|Damage|ApplyDamage OtherActor 1e+01 0 self "/Script/Engine.DamageType")
      (Collision|SetCollisionEnabled (Variables|Default|Getatk_hit_box) "NoCollision"))))

(event OnComponentBeginOverlap(Atk_rang)
  (params (OverlappedComponent :type Primitive%20Component%20Object%20Reference) (OtherActor :type Actor%20Object%20Reference) (OtherComp :type Primitive%20Component%20Object%20Reference) (OtherBodyIndex :type Integer) (bFromSweep :type Boolean) (SweepResult :type Hit%20Result%20Structure%20%28by%20ref%29))
  ;[1 1 1] in attack range
  (if (Actor|ActorHasTag OtherActor "player")
    (Variables|Default|Setin%20atk%20range true)))

(event OnComponentEndOverlap(Atk_rang)
  (params (OverlappedComponent :type Primitive%20Component%20Object%20Reference) (OtherActor :type Actor%20Object%20Reference) (OtherComp :type Primitive%20Component%20Object%20Reference) (OtherBodyIndex :type Integer))
  ;[1 1 1] in attack range
  (if (Actor|ActorHasTag OtherActor "player")
    (Variables|Default|Setin%20atk%20range false)))

(event OnComponentEndOverlap(findplayer)
  (params (OverlappedComponent :type Primitive%20Component%20Object%20Reference) (OtherActor :type Actor%20Object%20Reference) (OtherComp :type Primitive%20Component%20Object%20Reference) (OtherBodyIndex :type Integer))
  (if (Actor|ActorHasTag OtherActor "player")
    (Variables|Default|Setfind%20player? false)))

(event Game|Damage|EventAnyDamage
  (params (Damage :type Float%20%28single-precision%29) (DamageType :type Damage%20Type%20Object%20Reference) (InstigatedBy :type Controller%20Object%20Reference) (DamageCauser :type Actor%20Object%20Reference))
  ;[1 1 1] dmg input
  (if (Actor|ActorHasTag DamageCauser "player")
    (Variables|Default|Sethp (- (Variables|Default|Gethp) Damage))))

(event Collision|EventActorBeginOverlap
  (params (OtherActor :type Actor%20Object%20Reference)))

(event EventTick
  (params (DeltaSeconds :type Float%20%28single-precision%29))
  ;[1 1 1] check hp
  (if (> (Variables|Default|Gethp) 0.0)
    ;[1 1 1] check playing atk animation
    (if (Variables|Default|Getstop%20event)
      (Development|PrintString "aHello")
      (else
        (Development|PrintString "Hello")
        ;[1 1 1] check player is in collision
        (if (Variables|Default|Getfind%20player?)
          ;[1 1 1] check player is in atk range
          (if (Variables|Default|Getin%20atk%20range)
            ;[1 1 1] play atk animation and stop for 2 second
            (Class|SkinnedMeshComponent|SetMasterPoseComponent (Variables|Character|GetMesh) 0 false)
            (if (not (Variables|Default|Getatked?))
              (Variables|Default|Setstop%20event true)
              (Components|Animation|PlayAnimation (Variables|Default|GetHair) "/Game/QuadrapedCreatures/Barghest/Animations/BARGHEST_runBite_RM.BARGHEST_runBite_RM" false)
              (Variables|Default|Setatked? true)
              (Utilities|FlowControl|Delay 0.3)
              (Collision|SetCollisionEnabled (Variables|Default|Getatk_hit_box) "QueryAndPhysics")
              (Utilities|FlowControl|Delay 0.3)
              (Collision|SetCollisionEnabled (Variables|Default|Getatk_hit_box) "NoCollision")
              (Class|SkinnedMeshComponent|SetMasterPoseComponent (Variables|Character|GetMesh) 0 false)
              (Components|Animation|PlayAnimation (Variables|Default|GetHair) "/Game/QuadrapedCreatures/Barghest/Animations/BARGHEST_idleBreathe.BARGHEST_idleBreathe" false)
              (Utilities|FlowControl|Delay 2.0)
              (Variables|Default|Setstop%20event false)
              (Variables|Default|Setatked? false))
            (else
              ;[1 1 1] go to player's location
              (if (> (Variables|Default|Gethp) 0.0)
                (bind _ascharacter (Utilities|Casting|CastToCharacter (Game|Player|GetPlayerPawn 0)))
                (AI|AIMoveTo self "0, 0, 0" _ascharacter 5.0 false
                  (:then
                    (Class|SkinnedMeshComponent|SetMasterPoseComponent (Variables|Character|GetMesh) 0 false)
                    (Components|Animation|PlayAnimation (Variables|Default|GetHair) "/Game/QuadrapedCreatures/Barghest/Animations/BARGHEST_run.BARGHEST_run" true)
                    (Variables|Default|Setstop%20event true)
                    (Utilities|FlowControl|Delay 0.6)
                    (Variables|Default|Setstop%20event false))))))
          (else
            ;[1 1 1] random go around the navgation
            (Utilities|FlowControl|Delay (Math|Random|RandomFloatinRange 3.0 5.0))
            (if (> (Variables|Default|Gethp) 0.0)
              (AI|AIMoveTo self (.RandomLocation (AI|Navigation|GetRandomReachablePointinRadius (Transformation|GetActorLocation) 5e+03 0 0)) 0 5.0 false
                (:then
                  (Class|SkinnedMeshComponent|SetMasterPoseComponent (Variables|Character|GetMesh) 0 true)
                  (Components|Animation|PlayAnimation (Variables|Default|GetHair) "/Game/QuadrapedCreatures/Barghest/Animations/BARGHEST_run.BARGHEST_run" true))))))))
    (else
      ;[1 1 1] play dead animation
      (Class|SkinnedMeshComponent|SetMasterPoseComponent (Variables|Character|GetMesh) 0 false)
      (Components|Animation|PlayAnimation (Variables|Default|GetHair) "/Game/QuadrapedCreatures/Barghest/Animations/BARGHEST_deathNormal.BARGHEST_deathNormal" false)
      (Utilities|FlowControl|Delay 2.0)
      (Actor|DestroyActor))))

(fn ConstructionScript)