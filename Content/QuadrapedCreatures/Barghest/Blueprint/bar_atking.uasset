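; Anim notify state that marks the active hit window in the Barghest creature's attack animations.
; On begin it casts the mesh owner to Bp_Barghest and switches its AtkHitBox to query-only collision.
; On end it sets the same hitbox back to no collision, so the notify's span on the animation defines when the hitbox is live.
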(fn ReceivedNotifyBegin
  (params (MeshComp :type Skeletal%20Mesh%20Component%20Object%20Reference) (Animation :type Anim%20Sequence%20Base%20Object%20Reference) (TotalDuration :type Float%20%28single-precision%29))
  (Collision|SetCollisionEnabled (Variables|/Game/QuadrapedCreatures/Barghest/Blueprint/Bp_Barghest.Bp_Barghest_C|Getatk_hit_box (.AsBp%20Barghest (Utilities|Casting|CastToBp_Barghest (Components|GetOwner MeshComp)))) "QueryOnly")
  (return false))

(fn ReceivedNotifyEnd
  (params (MeshComp :type Skeletal%20Mesh%20Component%20Object%20Reference) (Animation :type Anim%20Sequence%20Base%20Object%20Reference))
  (Collision|SetCollisionEnabled (Variables|/Game/QuadrapedCreatures/Barghest/Blueprint/Bp_Barghest.Bp_Barghest_C|Getatk_hit_box (.AsBp%20Barghest (Utilities|Casting|CastToBp_Barghest (Components|GetOwner MeshComp)))) "NoCollision")
  (return false))