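; Mountain dragon creature Blueprint that wanders and tracks its health against player attacks.
; Tick uses a random Delay to pace AI moves to random reachable points around it.
; Damage from player-tagged causers lowers Hp and updates the HP bar widget, which shows while the player overlaps the FindPlayer volume.
; The runaway and DecideNextAction events are stubs: flee radius is zero and the decision branch is empty.
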(event OnComponentBeginOverlap(findplayer)
  (params (OverlappedComponent :type Primitive%20Component%20Object%20Reference) (OtherActor :type Actor%20Object%20Reference) (OtherComp :type Primitive%20Component%20Object%20Reference) (OtherBodyIndex :type Integer) (bFromSweep :type Boolean) (SweepResult :type Hit%20Result%20Structure%20%28by%20ref%29))
  (if (Actor|ActorHasTag OtherActor "player")
    ;[1 1 1] show hp bar
    (Variables|Default|Setfind%20player? true)
    (Rendering|SetVisibility (Variables|Default|GetHPBar) true false)))

(event OnComponentEndOverlap(findplayer)
  (params (OverlappedComponent :type Primitive%20Component%20Object%20Reference) (OtherActor :type Actor%20Object%20Reference) (OtherComp :type Primitive%20Component%20Object%20Reference) (OtherBodyIndex :type Integer))
  (if (Actor|ActorHasTag OtherActor "player")
    ;[1 1 1] show hp bar
    (Variables|Default|Setfind%20player? false)
    (Rendering|SetVisibility (Variables|Default|GetHPBar) false false)))

(event Custom|Decide%20Next%20Action
  (params (Skip%20delay? :type Boolean))
  (if Skip%20delay?
    _
    (else
      (Utilities|FlowControl|Delay (Math|Random|RandomFloatinRange 1.0 5.0))))
  (if true
    _))

(event Custom|run%20away
  ;[1 1 1] Run away
  (Variables|/Script/Engine.CharacterMovementComponent|SetMaxWalkSpeed (Variables|Character|GetCharacterMovement) 6e+02)
  (AI|AIMoveTo self (.RandomLocation (AI|Navigation|GetRandomReachablePointinRadius (Transformation|GetActorLocation) (Math|Random|RandomFloatinRange 0.0 0.0) 0 0)) 0 5.0 false
    (:OnSuccess
      (CallFunction|DecideNextAction true))))

(event Game|Damage|EventAnyDamage
  (params (Damage :type Float%20%28single-precision%29) (DamageType :type Damage%20Type%20Object%20Reference) (InstigatedBy :type Controller%20Object%20Reference) (DamageCauser :type Actor%20Object%20Reference))
  (if (Actor|ActorHasTag DamageCauser "player")
    (bind _output_get (Variables|Default|Sethp (- (Variables|Default|Gethp) Damage)))
    (Variables|/Game/QuadrapedCreatures/MountainDragon/blueprint/dragon_HPBar.dragon_HPBar_C|Sethp_bar (Variables|Default|GetAs%20Dragon%20HPBar) _output_get)
    (Development|PrintString (Utilities|String|Append "enemy hp :" (Utilities|String|ToString(Float) _output_get)))))

(event EventTick
  (params (DeltaSeconds :type Float%20%28single-precision%29))
  (Utilities|FlowControl|Delay (Math|Random|RandomFloatinRange 1.0 5.0))
  (AI|AIMoveTo self (.RandomLocation (AI|Navigation|GetRandomReachablePointinRadius (Transformation|GetActorLocation) 1e+04 0 0)) 0 5.0 false))

(event EventBeginPlay
  (bind _asdragon_hpbar (Utilities|Casting|CastTodragon_HPBar (UserInterface|GetUserWidgetObject (Variables|Default|GetHPBar))))
  (Variables|Default|SetAs%20Dragon%20HPBar _asdragon_hpbar))

(fn ConstructionScript)